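; Bird actor that flies along a referenced spline track while emitting bird sounds.
; MoveBirds starts a timeline, scaled by Duration and begun at StartOffset, whose alpha sets the actor's location and rotation by distance along TrackRef's spline.
; In parallel, it endlessly spawns a sound at Bird1's position, waits a random few seconds, fades it out and repeats.
; The Pause function is empty.
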(event Custom|MoveBirds
  (Utilities|FlowControl|Sequence
    (:then_0
      (bind _returnvalue (Audio|SpawnSoundatLocation "/Game/Blueprints/Sounds/Birds/MainBirds/BirdWAVChange_Cue.BirdWAVChange_Cue" (Transformation|GetWorldLocation (Variables|Default|Getbird1)) "0, 0, 0" 1.0 1.0 0.0 0 0 :!label _label))
      (Utilities|FlowControl|Delay (Math|Random|RandomFloatinRange 1.0 3.0))
      (Audio|Components|Audio|FadeOut _returnvalue 0.4 0.2 "Logarithmic" :!class /Script/Engine.AudioComponent)
      (goto _label))
    (:then_1
      (Components|Timeline|SetPlayRate (Variables|Default|Gettimeline) (/ 1.0 (Variables|Default|GetDuration)))
      (Components|Timeline|SetNewTime (Variables|Default|Gettimeline) (Variables|Default|GetStartOffset))
      (bind _alpha (Timeline|timeline Play)
        (:Update
          (Variables|Default|SetAlpha _alpha)
          (Transformation|SetActorLocationAndRotation (Spline|GetLocationatDistanceAlongSpline (Variables|/Game/Blueprints/birds_Track.birds_Track_C|GetSpline (Variables|Default|GetTrackRef)) (Math|Float|Lerp 0.0 (Spline|GetSplineLength (Variables|/Game/Blueprints/birds_Track.birds_Track_C|GetSpline (Variables|Default|GetTrackRef))) (Variables|Default|GetAlpha)) "World") (Spline|GetRotationatDistanceAlongSpline (Variables|/Game/Blueprints/birds_Track.birds_Track_C|GetSpline (Variables|Default|GetTrackRef)) (Math|Float|Lerp 0.0 (Spline|GetSplineLength (Variables|/Game/Blueprints/birds_Track.birds_Track_C|GetSpline (Variables|Default|GetTrackRef))) (Variables|Default|GetAlpha)) "World")))))))

(fn ConstructionScript)

(fn Pause)