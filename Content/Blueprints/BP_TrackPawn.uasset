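; BP_TrackPawn is a Blueprint that moves itself along the spline of a referenced track actor over a configurable total time.
; BeginPlay sets the timeline length to TotalTime, and the MoveAlongTrack event plays the timeline from the start.
; Each update divides playback position by TotalTime to sample a world-space spline location without constant velocity, then sets the actor's location, with no rotation input wired.
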(event Custom|Move%20Along%20Track
  (Timeline|Timeline_0 PlayFromStart
    (:Update
      (Transformation|SetActorLocationAndRotation (Spline|GetLocationatTime (Variables|/Game/Blueprints/BP_Track.BP_Track_C|GetSpline (Variables|Default|GetTrackRef)) (/ (Components|Timeline|GetPlaybackPosition (Variables|Default|GetTimeline_0)) (Variables|Default|GetTotal%20Time)) "World" false) "0, 0, 0"))))

(event EventBeginPlay
  (Components|Timeline|SetTimelineLength (Variables|Default|GetTimeline_0) (Variables|Default|GetTotal%20Time)))

(fn ConstructionScript)