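; LadyBug actor that travels along the spline of a referenced track actor.
; On BeginPlay, if ActivAnt is set, a timeline starts at StartOffset with a play rate derived from Duration.
; Its Alpha maps to distance along the spline, setting the bug's world location and rotation each update.
; Tick separately increments a Seconds counter through a one-second Delay, unused elsewhere in this graph.
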(event Custom|MoveLadyBug
  (Components|Timeline|SetPlayRate (Variables|Default|Gettimeline) (/ 1.0 (Variables|Default|GetDuration)))
  (Components|Timeline|SetNewTime (Variables|Default|Gettimeline) (Variables|Default|GetStartOffset))
  (bind _alpha (Timeline|timeline Play)
    (:Update
      (Variables|Default|SetAlpha _alpha)
      (Transformation|SetActorLocationAndRotation (Spline|GetLocationatDistanceAlongSpline (Variables|/Game/Blueprints/ladyBug_Track.ladyBug_Track_C|GetSpline (Variables|Default|GetTrackRef)) (Math|Float|Lerp 0.0 (Spline|GetSplineLength (Variables|/Game/Blueprints/ladyBug_Track.ladyBug_Track_C|GetSpline (Variables|Default|GetTrackRef))) (Variables|Default|GetAlpha)) "World") (Spline|GetRotationatDistanceAlongSpline (Variables|/Game/Blueprints/ladyBug_Track.ladyBug_Track_C|GetSpline (Variables|Default|GetTrackRef)) (Math|Float|Lerp 0.0 (Spline|GetSplineLength (Variables|/Game/Blueprints/ladyBug_Track.ladyBug_Track_C|GetSpline (Variables|Default|GetTrackRef))) (Variables|Default|GetAlpha)) "World")))))

(event EventBeginPlay
  ;[0 1 0.1514] Call moving function at start
  (if (Variables|Default|GetActiv%20Ant)
    (CallFunction|MoveLadyBug)))

(event EventTick
  (params (DeltaSeconds :type Float%20%28single-precision%29))
  (Utilities|FlowControl|Delay 1.0)
  (Variables|Default|Setseconds (+ (Variables|Default|Getseconds) 1)))

(fn ConstructionScript)