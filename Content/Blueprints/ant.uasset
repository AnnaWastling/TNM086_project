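; Ant actor that travels along the spline of a referenced track actor.
; The MoveAnt event scales a timeline's play rate by the inverse of Duration and starts it from a per-ant time offset.
; Each update maps the timeline alpha to a distance along the spline, then sets the ant's world location and rotation from that point.
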(event Custom|MoveAnt
  (Components|Timeline|SetPlayRate (Variables|Default|Gettimeline) (/ 1.0 (Variables|Default|GetDuration)))
  (Components|Timeline|SetNewTime (Variables|Default|Gettimeline) (Variables|Default|GetantStartOffset))
  (bind _alpha (Timeline|timeline Play)
    (:Update
      (Variables|Default|SetAlpha _alpha)
      (Transformation|SetActorLocationAndRotation (Spline|GetLocationatDistanceAlongSpline (Variables|/Game/Blueprints/Ant_Track.Ant_Track_C|GetSpline (Variables|Default|GetTrackRef)) (Math|Float|Lerp 0.0 (Spline|GetSplineLength (Variables|/Game/Blueprints/Ant_Track.Ant_Track_C|GetSpline (Variables|Default|GetTrackRef))) (Variables|Default|GetAlpha)) "World") (Spline|GetRotationatDistanceAlongSpline (Variables|/Game/Blueprints/Ant_Track.Ant_Track_C|GetSpline (Variables|Default|GetTrackRef)) (Math|Float|Lerp 0.0 (Spline|GetSplineLength (Variables|/Game/Blueprints/Ant_Track.Ant_Track_C|GetSpline (Variables|Default|GetTrackRef))) (Variables|Default|GetAlpha)) "World")))))

(fn ConstructionScript)