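; BP_TrackPawn travels along the spline of a referenced track in the dome camera setup, with bird ambience around it.
; If Active, it plays a timeline with rate set by Duration and start time by Offset, mapping Alpha to spline distance for position and rotation.
; Independently of Active, a delay loop plays attenuated bird sounds at randomly offset positions near the pawn every few seconds.
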(event Custom|Move%20Along%20Track
  (Components|Timeline|SetPlayRate (Variables|Default|GetTimeline_1) (/ 1.0 (Variables|Default|GetDuration)))
  (Components|Timeline|SetNewTime (Variables|Default|GetTimeline_1) (Variables|Default|GetOffset))
  (bind _alpha (Timeline|Timeline_1 Play)
    (:Update
      (Variables|Default|SetAlpha _alpha)
      (Transformation|SetActorLocationAndRotation (Spline|GetLocationatDistanceAlongSpline (Variables|/Game/Blueprints/DomeCamera/BP_Track.BP_Track_C|GetSpline (Variables|Default|GetTrackRef)) (Math|Float|Lerp 0.0 (Spline|GetSplineLength (Variables|/Game/Blueprints/DomeCamera/BP_Track.BP_Track_C|GetSpline (Variables|Default|GetTrackRef))) (Variables|Default|GetAlpha)) "World") (Spline|GetRotationatDistanceAlongSpline (Variables|/Game/Blueprints/DomeCamera/BP_Track.BP_Track_C|GetSpline (Variables|Default|GetTrackRef)) (Math|Float|Lerp 0.0 (Spline|GetSplineLength (Variables|/Game/Blueprints/DomeCamera/BP_Track.BP_Track_C|GetSpline (Variables|Default|GetTrackRef))) (Variables|Default|GetAlpha)) "World")))))

(event EventBeginPlay
  ;[0 1 0.4373] Start movement
  (Utilities|FlowControl|Sequence
    (:then_0
      (if (Variables|Default|GetActive)
        (CallFunction|MoveAlongTrack)))
    (:then_1
      (Audio|PlaySoundatLocation "/Game/Blueprints/Sounds/Birds/Ambient/AlBirds.AlBirds" (+ (Transformation|GetActorLocation) (Math|Random|RandomFloatinRange -1e+03 1e+03)) "0, 0, 0" 1.0 1.0 0.0 "/Game/Blueprints/Sounds/Birds/Ambient/AlBirdsAtteniation.AlBirdsAtteniation" 0 0 :!label _label)
      (Utilities|FlowControl|Delay (Math|Random|RandomFloatinRange 3.0 1e+01))
      (goto _label))))

(fn ConstructionScript)