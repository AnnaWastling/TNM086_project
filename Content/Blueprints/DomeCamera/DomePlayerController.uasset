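; Player controller for the dome camera that manages possession of a default BP_TrackPawn and resets its view.
; On BeginPlay it caches the controlled track pawn, its location and the control rotation.
; ResetView teleports the pawn back, restores that rotation and repossesses it.
; Input_One repossesses the pawn after DisableInputs loops over AlignedActors, disabling each one's input and unpossessing.
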(event EventBeginPlay
  ;[0 0.1339 1] Setup of initial values
  (bind _asbp_track_pawn (Utilities|Casting|CastToBP_TrackPawn (Pawn|GetControlledPawn)))
  (bind _output_get (Variables|Default|SetDefaultPawn _asbp_track_pawn))
  (Variables|Default|SetOriginPos (Transformation|GetActorLocation _output_get))
  (Variables|Default|SetOriginRot (Pawn|GetControlRotation :!class /Script/Engine.Controller)))

(event Input|ActionEvents|InputActionResetView
  (params (Key :type Key%20Structure :default "None"))
  ;[0 1 0.997] Resetting the view with the initial values
  (:Released
    (Transformation|SetActorLocation (Variables|Default|GetDefaultPawn) (Variables|Default|GetOriginPos) false true)
    (Pawn|SetControlRotation (Variables|Default|GetOriginRot))
    (Pawn|Possess (Variables|Default|GetDefaultPawn))))

(event Input|ActionEvents|InputActionInput_One
  (params (Key :type Key%20Structure :default "None"))
  ;[0.02316 0.6432 1] Add Input one
  (:Pressed
    (CallFunction|DisableInputs)
    (Pawn|Possess (Variables|Default|GetDefaultPawn))))

(fn ConstructionScript)

(fn DisableInputs
  (for _array_element (Variables|Default|GetAlignedActors)
    (Input|DisableInput _array_element self)
    (Pawn|UnPossess)))