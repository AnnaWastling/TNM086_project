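; Ant actor that travels along the spline of a referenced track actor.
; On BeginPlay, if the ant is flagged active, it plays a timeline scaled to a set duration and started at a per-ant offset.
; Each timeline update maps alpha to distance along the spline and sets the actor's world location and rotation to match.
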(event Custom|MoveAnt
  (Components|Timeline|SetPlayRate (Variables|Default|GetAntMover) (/ 1.0 (Variables|Default|GetDuration)))
  (Components|Timeline|SetNewTime (Variables|Default|GetAntMover) (Variables|Default|GetantStartOffset))
  (bind _alpha (Timeline|AntMover Play)
    (:Update
      (Variables|Default|SetAlpha _alpha)
      (Transformation|SetActorLocationAndRotation (Spline|GetLocationatDistanceAlongSpline (Variables|/Game/Blueprints/Ant_Track.Ant_Track_C|GetSpline (Variables|Default|GetTrackRef)) (Math|Float|Lerp 0.0 (Spline|GetSplineLength (Variables|/Game/Blueprints/Ant_Track.Ant_Track_C|GetSpline (Variables|Default|GetTrackRef))) (Variables|Default|GetAlpha)) "World") (Spline|GetRotationatDistanceAlongSpline (Variables|/Game/Blueprints/Ant_Track.Ant_Track_C|GetSpline (Variables|Default|GetTrackRef)) (Math|Float|Lerp 0.0 (Spline|GetSplineLength (Variables|/Game/Blueprints/Ant_Track.Ant_Track_C|GetSpline (Variables|Default|GetTrackRef))) (Variables|Default|GetAlpha)) "World")))))

(event EventBeginPlay
  (if (Variables|Default|GetActiv%20Ant)
    (CallFunction|MoveAnt)))

(fn ConstructionScript)