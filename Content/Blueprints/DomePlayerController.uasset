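; DomePlayerController is a player controller that hands input to actors held in its AlignedActors array.
; Pressing Input_Two calls DisableInputs, which loops over the array, disabling each actor's input and calling UnPossess on every iteration.
; It then re-enables input on the first actor in the array.
; Initial setup, view reset and the first and third inputs exist only as comments or empty events.
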(event EventBeginPlay
  ;[0 0.1339 1] Setup of initial values
)

(event Input|ActionEvents|InputActionInput_One
  (params (Key :type Key%20Structure :default "None"))
  ;[0.02316 0.6432 1] Add Input one
)

(event Input|ActionEvents|InputActionInput_Two
  (params (Key :type Key%20Structure :default "None"))
  ;[0 1 0.4685] Add Input 2
  (:Pressed
    (CallFunction|DisableInputs)
    (if (> (Utilities|Array|Length (Variables|Default|GetAligned%20Actors)) 0)
      (Input|EnableInput (Utilities|Array|Get(acopy) (Variables|Default|GetAligned%20Actors)) self))))

(event Input|ActionEvents|InputActionInput_Three
  (params (Key :type Key%20Structure :default "None"))
  ;[1 0.4349 0] Add input 3
)

(event Input|ActionEvents|InputActionResetView
  (params (Key :type Key%20Structure :default "None"))
  ;[0 1 0.997] Resetting the view with the initial values
)

(fn ConstructionScript)

(fn DisableInputs
  (for _array_element (Variables|Default|GetAligned%20Actors)
    (Input|DisableInput _array_element self)
    (Pawn|UnPossess)))